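; AC_Player is a player component that tracks the Coins and Stars stats.
; UpdateStats takes an add flag, an amount and a stat selector, negates the amount when not adding, and applies it to the chosen counter.
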(fn `UpdateStats`
  (params (`Add?` :type Boolean) (Amount :type Integer) (Stats :type "/Game/BaseGame/E_Stats Enum" :default "NewEnumerator0"))
  (locals (FinalAmount :type Integer))
  (if `Add?`
    (set `local.FinalAmount` Amount)
    (else
      (set `local.FinalAmount` (* Amount -1))))
  (switch `/Game/BaseGame/E_Stats` Stats
    (:`NewEnumerator0`
      (set `self.Coins` (+ (`self.Coins`) (`local.FinalAmount`))))
    (:`NewEnumerator1`
      (set `self.Stars` (+ (`self.Stars`) (`local.FinalAmount`))))))