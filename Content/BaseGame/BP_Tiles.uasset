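; BP_Tiles is a tile actor that adjusts a player's coins according to its TileTypes value.
; Overlapping TileCollision fires LandedOnTile, which passes the actor and tile type to TileFunctionality.
; That function calls UpdateCoinsMessage on the actor, adding coins for Blue and removing them for Red.
; Per-type textures are still pending, with only a reminder print on BeginPlay for Blue tiles.
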(event `self.ReceiveBeginPlay`
  (switch `/Game/BaseGame/E_TileTypes` (`self.TileTypes`)
    (:`NewEnumerator0`
      (`KismetSystemLibrary.PrintString` "NEED TO CHANGE THE TEXTURES TO THEIR RESPECTIVE TILE"))))

(event `LandedOnTile`
  (params (`Interacting Player` :type "Actor Object Reference"))
  (`self.TileFunctionality` `Interacting Player` (`self.TileTypes`)))

(event `self.TileCollision.OnComponentBeginOverlap`
  (params (OverlappedComponent :type "PrimitiveComponent Object Reference") (OtherActor :type "Actor Object Reference") (OtherComp :type "PrimitiveComponent Object Reference") (OtherBodyIndex :type Integer) (bFromSweep :type Boolean) (SweepResult :type "HitResult Structure (by ref)"))
  (`self.LandedOnTile` OtherActor))

(fn `TileFunctionality`
  (params (InteractingPlayer :type "Actor Object Reference") (TileType :type "/Game/BaseGame/E_TileTypes Enum" :default "NewEnumerator0"))
  (switch `/Game/BaseGame/E_TileTypes` TileType
    (:`NewEnumerator0`
      (`KismetSystemLibrary.PrintString` (`KismetSystemLibrary.GetDisplayName` InteractingPlayer))
      (message `/Game/BaseGame/BPI_Tiles.UpdateCoins` InteractingPlayer true 3))
    (:`NewEnumerator1`
      (message `/Game/BaseGame/BPI_Tiles.UpdateCoins` InteractingPlayer false 3))))

(fn `UserConstructionScript`)